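; A day and night cycle Blueprint that moves the sun over a configurable day length in minutes.
; BeginPlay converts that length into seconds per in-game hour, which Tick uses to advance an unwrapped hour counter.
; Each Tick maps the hour to sun pitch at 90 degrees per hour, offset by 90, then updates the sky dome's sun direction.
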(event `self.ReceiveBeginPlay`
  (bind _output_get (set `self.Oneday` (* (`self.daylengthinminutes`) 60.0)))
  (set `self.Onehour` (/ _output_get 24.0)))

(event `self.ReceiveActorBeginOverlap`
  (params (OtherActor :type "Actor Object Reference")))

(event `self.ReceiveTick`
  (params (DeltaSeconds :type "Float (single-precision)"))
  (bind _output_get (set `self.hour` (+ (`self.hour`) (/ DeltaSeconds (`self.Onehour`)))))
  (bind _output_get_2 (set `self.sunangle` (+ (* (/ _output_get 1.0) 90.0) 90.0)))
  (`self.SetActorRotation` (`self.sun`) (`KismetMathLibrary.MakeRotator` 0.0 _output_get_2))
  (`/Engine/EngineSky/BP_Sky_Sphere.UpdateSunDirection` (`self.skydome`)))

(fn `UserConstructionScript`)